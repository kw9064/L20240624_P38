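; Player-controlled P-38 aircraft pawn with simple arcade-style flight.
; Pitch and Roll axis inputs rotate the actor locally at a clamped, frame-rate-independent rate, with no yaw control.
; Tick constantly adds movement input along the forward vector, so steering comes entirely from orientation.
; The WEP action acts as a booster, raising the movement scale to full while held and dropping it to half on release.
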(event `InputAxis|Pitch`
  (params (AxisValue :type "Float (single-precision)"))
  ;[1 1 1] Pitch
  (`self.K2_AddActorLocalRotation` (`KismetMathLibrary.MakeRotator` 0.0 (* (`KismetMathLibrary.FClamp` AxisValue -1.0) 60.0 (`GameplayStatics.GetWorldDeltaSeconds`)))))

(event `InputAxis|Roll`
  (params (AxisValue :type "Float (single-precision)"))
  ;[1 1 1] Roll
  (`self.K2_AddActorLocalRotation` (`KismetMathLibrary.MakeRotator` (* (`KismetMathLibrary.FClamp` AxisValue -1.0) 60.0 (`GameplayStatics.GetWorldDeltaSeconds`)))))

(event `self.ReceiveTick`
  (params (DeltaSeconds :type "Float (single-precision)"))
  ;[1 1 1] MoveForward
  (`self.AddMovementInput` (`self.GetActorForwardVector`) (`self.Scale Value`)))

(event `InputAction|WEP`
  (params (Key :type "Key Structure"))
  ;[1 1 1] Booster
  (:`Pressed`
    (set `self.Scale Value` 1.0))
  (:`Released`
    (set `self.Scale Value` 0.5)))

(fn `UserConstructionScript`)